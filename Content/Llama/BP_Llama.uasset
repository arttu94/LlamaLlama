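; BP_Llama is a llama actor that takes damage over time while its replicated state is On Fire.
; On the authority, Tick accumulates delta time and calls a server damage event about once a second, which damages the llama and resets the timer.
; AnyDamage subtracts the truncated damage from Health and prints it.
; BeginPlay stores a dynamic material, but nothing uses it yet, and the state's OnRep is empty.
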(event Custom|Server_DamageLlama
  (params (BaseDamage :type Float%20%28single-precision%29))
  (bind _self self)
  (Game|Damage|ApplyDamage _self BaseDamage 0 _self)
  (Variables|Default|SetDamageDeltaTime 0.0))

(event EventBeginPlay
  (bind _returnvalue (Rendering|Material|CreateDynamicMaterialInstance (Variables|Character|GetMesh) 0 "/Game/Llama/Material/Llama.Llama" "None" :!class /Script/Engine.PrimitiveComponent))
  (Variables|Default|SetLlamaMat _returnvalue))

(event Collision|EventActorBeginOverlap
  (params (OtherActor :type Actor%20Object%20Reference)))

(event EventTick
  (params (DeltaSeconds :type Float%20%28single-precision%29))
  (Networking|SwitchHasAuthority
    (:Authority
      (switch Utilities|FlowControl|Switch|SwitchonLlamaState (Variables|Default|GetllamaState)
        (:NewEnumerator3
          (bind _output_get (Variables|Default|SetDamageDeltaTime (+ DeltaSeconds (Variables|Default|GetDamageDeltaTime))))
          (if (>= _output_get 1.0)
            (CallFunction|ServerDamageLlama 2.0)))))))

(event Game|Damage|EventAnyDamage
  (params (Damage :type Float%20%28single-precision%29) (DamageType :type Damage%20Type%20Object%20Reference) (InstigatedBy :type Controller%20Object%20Reference) (DamageCauser :type Actor%20Object%20Reference))
  (bind _output_get (Variables|Default|SetHealth (- (Variables|Default|GetHealth) (Math|Float|Truncate Damage))))
  (Development|PrintString (Utilities|String|ToString(Integer) _output_get)))

(fn ConstructionScript)

(fn OnRepLlamaState)