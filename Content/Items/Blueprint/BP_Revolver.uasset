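; Revolver item for a llama Carrier, with a primary action that only plays a montage and a Russian-roulette secondary action.
; The secondary randomly either ragdolls and damages the carrier or plays a fail montage, then requires a reload either way.
; The next secondary action plays the reload, cleared by a ReloadEnd notify or the multicast montage's blend-out.
; Multicast events replay montages and the ragdoll across the network.
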(event Custom|Multicast_PrimaryAction
  (bind _carrier (Variables|Default|Getcarrier))
  (Utilities|IsValid _carrier
    (:Is%20Valid
      (Animation|PlayAnimMontage _carrier "/Game/Llama/Animation/Anim_Llama_Revolver_Primary_Montage.Anim_Llama_Revolver_Primary_Montage" 1.0 "None"))))

(event Custom|Multicast_SecondaryAction
  (params (Fail? :type Boolean))
  (bind _carrier (Variables|Default|Getcarrier))
  (Utilities|IsValid _carrier
    (:Is%20Valid
      (if Fail?
        (Animation|PlayAnimMontage _carrier "/Game/Llama/Animation/Anim_Llama_Revolver_SecondaryFail_Montage.Anim_Llama_Revolver_SecondaryFail_Montage" 2.0 "None")
        (else
          (Animation|PlayAnimMontage _carrier "/Game/Llama/Animation/Anim_Llama_Revolver_Secondary_Montage.Anim_Llama_Revolver_Secondary_Montage" 2.0 "None")
          (Physics|SetSimulatePhysics (Variables|/Script/Engine.Character|GetMesh _carrier) true))))))

(event Custom|Multicast_Reload
  (Animation|Montage|PlayMontage (Variables|/Script/Engine.Character|GetMesh (Variables|Default|Getcarrier)) "/Game/Llama/Animation/Anim_Llama_Revolver_Reload_Montage.Anim_Llama_Revolver_Reload_Montage"
    (:OnBlendOut
      (Variables|Default|SetneedsReload? false))))

(event EventBeginPlay)

(event Collision|EventActorBeginOverlap
  (params (OtherActor :type Actor%20Object%20Reference)))

(event EventTick
  (params (DeltaSeconds :type Float%20%28single-precision%29)))

(event EventOnPrimaryAction
  (bind _carrier (Variables|Default|Getcarrier))
  (Utilities|IsValid _carrier
    (:Is%20Valid
      (Animation|PlayAnimMontage _carrier "/Game/Llama/Animation/Anim_Llama_Revolver_Primary_Montage.Anim_Llama_Revolver_Primary_Montage" 2.0 "None")
      (CallFunction|MulticastPrimaryAction))))

(event EventOnSecondaryAction
  (bind _carrier (Variables|Default|Getcarrier))
  (if (Variables|Default|GetneedsReload?)
    (bind _notifyname (Animation|Montage|PlayMontage (Variables|/Script/Engine.Character|GetMesh (Variables|Default|Getcarrier)) "/Game/Llama/Animation/Anim_Llama_Revolver_Reload_Montage.Anim_Llama_Revolver_Reload_Montage")
      (:then
        (CallFunction|MulticastReload))
      (:OnNotifyBegin
        (if (Utilities|Name|Equal(Name) _notifyname "ReloadEnd")
          (Variables|Default|SetneedsReload? false))))
    (else
      (Utilities|IsValid _carrier
        (:Is%20Valid
          (if (== 0 (Math|Random|RandomInteger 6))
            (Animation|PlayAnimMontage _carrier "/Game/Llama/Animation/Anim_Llama_Revolver_Secondary_Montage.Anim_Llama_Revolver_Secondary_Montage" 2.0 "None")
            (Physics|SetSimulatePhysics (Variables|/Script/Engine.Character|GetMesh _carrier) true)
            (bind _asbp_llama (Utilities|Casting|CastToBP_Llama (Variables|Default|Getcarrier)))
            (Game|Damage|ApplyDamage _asbp_llama 5e+01 0 _asbp_llama)
            (Development|PrintString (Utilities|String|ToString(Integer) (Variables|/Game/Llama/BP_Llama.BP_Llama_C|GetHealth _asbp_llama)))
            (Variables|Default|SetneedsReload? true)
            (CallFunction|MulticastSecondaryAction false)
            (else
              (Animation|PlayAnimMontage _carrier "/Game/Llama/Animation/Anim_Llama_Revolver_SecondaryFail_Montage.Anim_Llama_Revolver_SecondaryFail_Montage" 2.0 "None")
              (CallFunction|MulticastSecondaryAction true)
              (Variables|Default|SetneedsReload? true))))))))

(fn ConstructionScript)