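; BP_Matches is a carried item that sets its llama carrier on fire when used.
; Its primary action checks the llama is in a specific state, plays a generic-use montage, switches the state and calls a multicast FX event.
; That event attaches a fire emitter to the carrier's mesh, replays the montage and sets the material's Burnt and Wet parameters.
; The looping fire sound is disconnected and never plays.
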(event Custom|Multicast_FireFX
  (bind _carrier (Variables|Default|Getcarrier))
  (bind _returnvalue (Effects|SpawnEmitterAttached "/Game/Effects/Fire_01.Fire_01" (Variables|/Script/Engine.Character|GetMesh _carrier) "" "0, 0,50.000000" "0, 0, 0" "1.000000,1.000000,1.000000" "SnapToTarget" false))
  (Animation|PlayAnimMontage _carrier "/Game/Llama/Animation/Anim_Llama_GenericUse_Montage.Anim_Llama_GenericUse_Montage" 1.0 "None")
  (bind _asbp_llama (Utilities|Casting|CastToBP_Llama (Variables|Default|Getcarrier)))
  (Rendering|Material|SetScalarParameterValue (Variables|/Game/Llama/BP_Llama.BP_Llama_C|GetLlamaMat _asbp_llama) "Burnt" 1.0 :!class /Script/Engine.MaterialInstanceDynamic)
  (Rendering|Material|SetScalarParameterValue (Variables|/Game/Llama/BP_Llama.BP_Llama_C|GetLlamaMat _asbp_llama) "Wet" 1.0 :!class /Script/Engine.MaterialInstanceDynamic))

(event EventBeginPlay)

(event Collision|EventActorBeginOverlap
  (params (OtherActor :type Actor%20Object%20Reference)))

(event EventTick
  (params (DeltaSeconds :type Float%20%28single-precision%29)))

(event EventOnPrimaryAction
  (bind _carrier (Variables|Default|Getcarrier))
  (Utilities|IsValid _carrier
    (:Is%20Valid
      (bind _asbp_llama (Utilities|Casting|CastToBP_Llama _carrier))
      (if (Utilities|Enum|Equal(Enum) (Variables|/Game/Llama/BP_Llama.BP_Llama_C|GetllamaState _asbp_llama) "NewEnumerator0")
        (Animation|PlayAnimMontage _asbp_llama "/Game/Llama/Animation/Anim_Llama_GenericUse_Montage.Anim_Llama_GenericUse_Montage" 1.0 "None")
        (Variables|/Game/Llama/BP_Llama.BP_Llama_C|SetllamaState _asbp_llama "NewEnumerator3")
        (CallFunction|MulticastFireFX)))))

(fn ConstructionScript)